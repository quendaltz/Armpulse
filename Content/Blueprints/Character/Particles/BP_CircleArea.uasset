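; Circle area decal actor that shows an area animating over a set Duration, then spawns an emitter at its location and destroys itself.
; SpawnCircleDecal creates dynamic materials for Circumference and Area, using the CircumArea parameter to differentiate ring and interior.
; A timeline with play rate scaled by 1/Duration drives the Area's AreaValue, with short delays before and after.
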(event `self.ReceiveBeginPlay`)

(event `self.SpawnCircleDecal`
  ; Spawn Circle Decal
  (`TimelineComponent.SetPlayRate` (`self.AreaValueTimeline`) (`KismetMathLibrary.SafeDivide` 1.0 (`self.Duration`)))
  (`|ExecutionSequence`
    (:`then_0`
      (bind _returnvalue (`DecalComponent.CreateDynamicMaterialInstance` (`self.Circumference`)))
      (bind _output_get (set `self.CircumRef` _returnvalue))
      (`MaterialInstanceDynamic.SetScalarParameterValue` _output_get "CircumArea" 1.0))
    (:`then_1`
      (bind _returnvalue_2 (`DecalComponent.CreateDynamicMaterialInstance` (`self.Area`)))
      (bind _output_get_2 (set `self.AreaRef` _returnvalue_2))
      (`MaterialInstanceDynamic.SetScalarParameterValue` _output_get_2 "CircumArea" 0.0))
    (:`then_2`
      (`KismetSystemLibrary.Delay` 0.2)
      (bind (_direction _areavaluealpha) (`Timeline|AreaValueTimeline`)
        (:`Update`
          (`MaterialInstanceDynamic.SetScalarParameterValue` (`self.AreaRef`) "AreaValue" _areavaluealpha))
        (:`Finished`
          (`KismetSystemLibrary.Delay` 0.2)
          (`GameplayStatics.SpawnEmitterAtLocation` null (`self.K2_GetActorLocation`))
          (`self.K2_DestroyActor`))))))

(fn `UserConstructionScript`)